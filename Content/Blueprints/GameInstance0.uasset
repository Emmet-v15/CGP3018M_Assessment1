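; Game instance that tracks how many artifacts the player has collected out of three.
; IncrementCounter raises the count, plays a claim sound and rewrites the text of the first TextRenderActor found in the level to show progress.
; Once three are collected, that text becomes a congratulations message and a victory sound plays.
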(event EventInit)

(fn IncrementCounter
  ;[0.15 0.15 0.15 0.5] Increment Counter
  (Variables|Default|SetCounter (+ (Variables|Default|GetCounter) 1))
  (Audio|PlaySound2D "/Game/Sounds/claim-artifact.claim-artifact" 1.0 1.0 0.0 0 0)
  ;[0.15 0.15 0.15 0.5] Update Pedestal Text
  (bind _outactors (Actor|GetAllActorsOfClass "/Script/Engine.TextRenderActor"))
  (if (>= (Variables|Default|GetCounter) 3)
    (Rendering|Components|TextRender|SetText (Variables|/Script/Engine.TextRenderActor|GetTextRender (Utilities|Array|Get(acopy) _outactors)) (Utilities|Text|MakeLiteralText "Congratulations! 
You have collected all the Artifacts."))
    (Audio|PlaySound2D "/Game/Sounds/victory.victory" 1.0 1.0 0.0 0 0)
    (else
      (Rendering|Components|TextRender|SetText (Variables|/Script/Engine.TextRenderActor|GetTextRender (Utilities|Array|Get(acopy) _outactors)) (Utilities|Text|ToText(String) (Utilities|String|Append "Collect All the Artifacts! 
(" (Utilities|String|ToString(Integer) (Variables|Default|GetCounter)) "/3)"))))))