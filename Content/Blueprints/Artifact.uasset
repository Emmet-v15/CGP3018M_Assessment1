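; Artifact component that spins and bobs its parent component and acts as a one-time collectible for the player.
; Each Tick applies time-accumulated spin and sine bob offsets to the parent transform cached at BeginPlay.
; Tick also polls the owner's sphere for player pawn overlap, incrementing the GameInstance0 counter on first claim.
; Claiming replaces the cached transform with ClaimedLocation's, so the artifact keeps animating on its pedestal.
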(event EventBeginPlay
  ;[0.15 0.15 0.15 0.5] Create a transform copy
  (bind _output_get (Variables|Default|SetDefault%20Transform (Transformation|GetWorldTransform (Transformation|GetAttachParent)))))

(event EventTick
  (params (DeltaSeconds :type Float%20%28single-precision%29))
  ;[0.15 0.15 0.15 0.5] Apply offsets
  (bind _spin_offset (Utilities|CreateSpinOffset DeltaSeconds))
  (bind _bob_offset (Utilities|CreateBobOffset DeltaSeconds))
  (Transformation|SetWorldTransform (Transformation|GetAttachParent) (Math|Transform|MakeTransform (+ _bob_offset (.Location (Math|Transform|BreakTransform (stale EventBeginPlay _output_get)))) (Math|Rotator|CombineRotators (.Rotation (Math|Transform|BreakTransform (stale EventBeginPlay _output_get))) _spin_offset) (.Scale (Math|Transform|BreakTransform (stale EventBeginPlay _output_get)))) false false)
  ;[0.15 0.15 0.15 0.5] Increment Artifact counter on collision
  (if (Utilities|Array|ContainsItem (Collision|GetOverlappingActors (Actor|GetComponentbyClass (Components|GetOwner) "/Script/Engine.SphereComponent") 0 :!class /Script/Engine.PrimitiveComponent) (Game|Player|GetPlayerPawn 0))
    (if (not (Variables|Default|GetClaimed))
      (Variables|Default|SetClaimed true)
      (bind _asgame_instance_0 (Utilities|Casting|CastToGameInstance0 (Game|GetGameInstance)))
      (Default|IncrementCounter _asgame_instance_0)
      (Development|PrintString "Hello")
      ;[0.15 0.15 0.15 0.5] Move Artifact to pedestal
      (Variables|Default|SetDefault%20Transform (Transformation|GetActorTransform (Variables|Default|GetClaimed%20Location))))))