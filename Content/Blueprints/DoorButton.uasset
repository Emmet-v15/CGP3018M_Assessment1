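; DoorButton is a component that turns its owner into a clickable button that removes a linked door.
; On BeginPlay it creates a dynamic material instance from the first material slot of the owner's static mesh.
; A click sets the Colour parameter to the pressed color, waits briefly, restores the idle color, then destroys the Door actor and plays a 2D beep if that door is still valid.
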(event EventBeginPlay
  (bind _returnvalue (Components|GetOwner))
  (bind _returnvalue_2 (Actor|GetComponentbyClass _returnvalue "/Script/Engine.StaticMeshComponent"))
  ;[0.15 0.15 0.15 0.5] Prepare a dynamic material instance
  (bind _returnvalue_3 (Rendering|Material|CreateDynamicMaterialInstance _returnvalue_2 0 (Rendering|Material|GetMaterial _returnvalue_2 0) "None" :!class /Script/Engine.PrimitiveComponent))
  (Variables|Default|SetMaterial%20Instance _returnvalue_3))

(event EventOnClicked
  (bind _door (Variables|Default|GetDoor))
  ;[0.15 0.15 0.15 0.5] Handle Click
  (Rendering|Material|SetVectorParameterValue (Variables|Default|GetMaterial%20Instance) "Colour" (Variables|Default|GetPressedColor) :!class /Script/Engine.MaterialInstanceDynamic)
  (Utilities|FlowControl|Delay 1.0)
  (Rendering|Material|SetVectorParameterValue (Variables|Default|GetMaterial%20Instance) "Colour" (Variables|Default|GetIdleColor) :!class /Script/Engine.MaterialInstanceDynamic)
  (Utilities|IsValid _door
    (:Is%20Valid
      (Actor|DestroyActor _door)
      (Audio|PlaySound2D "/Game/Sounds/beep.beep" 1.0 1.0 0.0 0 0))))