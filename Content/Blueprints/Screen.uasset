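; Screen component for a rapid-click puzzle that rewards the player with a Penrose triangle artifact.
; Each click raises a counter and plays a beep pitched by it, while Tick drains the counter and tints the owner's dynamic mesh material from it.
; Once the counter reaches its threshold, a one-shot flag guards a glitch sound and the artifact spawn, with its claimed location set to the tagged pedestal.
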(event EventTick
  (params (DeltaSeconds :type Float%20%28single-precision%29))
  ;[0.15 0.15 0.15 0.5] Subtract 5 from counter every second
  (if (< (Variables|Default|GetCounter) 1e+01)
    (Variables|Default|SetCounter (Math|Float|Clamp(Float) (- (Variables|Default|GetCounter) (* DeltaSeconds 5.0)) 0.0 1e+01))
    ;[0.15 0.15 0.15 0.5] Set Material colour depending on counter
    (Rendering|Material|SetVectorParameterValue (Variables|Default|GetMaterialInstance) "Colour" (Math|Color|Lerp(LinearColor) (Variables|Default|GetIdle%20Color) (Variables|Default|GetActivated%20Color) (Variables|Default|GetCounter)) :!class /Script/Engine.MaterialInstanceDynamic)
    (else
      ;[0.15 0.15 0.15 0.5] Spawn Artifact
      ;;[0.15 0.15 0.15 0.5] Debounce
      (if (not (Variables|Default|GetFinished))
        (Variables|Default|SetFinished true)
        (Audio|PlaySoundatLocation "/Game/Sounds/glitch.glitch" (.Location (Math|Transform|BreakTransform (Transformation|GetActorTransform (Components|GetOwner)))) "0, 0, 0" 1.0 1.0 0.0 0 0 0 0)
        (bind _returnvalue (Game|SpawnActorfromClass "/Game/Blueprints/Penrose-Triangle.Penrose-Triangle_C" (Transformation|GetActorTransform (Variables|Default|GetArtifact%20Spawnpoint)) "Undefined" "MultiplyWithRoot" 0 0))
        (bind _outactors (Actor|GetAllActorswithTag "penrosePedistal"))
        (Variables|/Game/Blueprints/Artifact.Artifact_C|SetClaimed%20Location (Actor|GetComponentbyClass _returnvalue "/Game/Blueprints/Artifact.Artifact_C") (Utilities|Array|Get(acopy) _outactors))))))

(event EventBeginPlay
  (bind _returnvalue (Components|GetOwner))
  (bind _returnvalue_2 (Actor|GetComponentbyClass _returnvalue "/Script/Engine.StaticMeshComponent"))
  ;[0.15 0.15 0.15 0.5] Prepare a dynamic material instance
  (bind _returnvalue_3 (Rendering|Material|CreateDynamicMaterialInstance _returnvalue_2 0 (Rendering|Material|GetMaterial _returnvalue_2 0) "None" :!class /Script/Engine.PrimitiveComponent))
  (Variables|Default|SetMaterialInstance _returnvalue_3))

(event EventOnClicked
  ;[0.15 0.15 0.15 0.5] Add 1 to counter on click
  (bind _output_get (Variables|Default|SetCounter (+ (Variables|Default|GetCounter) 1.0)))
  (Audio|PlaySound2D "/Game/Sounds/beep.beep" 1.0 (/ _output_get 5.0) 0.0 0 0))